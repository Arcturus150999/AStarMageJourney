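; BP_DeathZone is a kill volume that kills the player and rolls back unsaved star coin pickups.
; Death collision overlaps re-show hidden, unsaved BP_StarCoins and restore their collision before the character cast, then call DeathPlayer and briefly pulse a Respawn flag.
; A separate dissolve collision plays a timeline that lowers gravity scale, overrides vertical velocity and drives the character's Dissolve material parameter.
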(event OnComponentBeginOverlap(DeathCollision)
  (params (OverlappedComponent :type Primitive%20Component%20Object%20Reference) (OtherActor :type Actor%20Object%20Reference) (OtherComp :type Primitive%20Component%20Object%20Reference) (OtherBodyIndex :type Integer) (bFromSweep :type Boolean) (SweepResult :type Hit%20Result%20Structure%20%28by%20ref%29))
  (bind _outactors (Actor|GetAllActorsOfClass "/Game/PersoFolder/BP/StarCoins/BP_StarCoins.BP_StarCoins_C"))
  (for _array_element _outactors
    ;[1 1 1] Permet de cacher la sphere si elle a été récupéré et que le joueur est passé sur un checkpoint
    (if (Variables|/Script/Engine.Actor|GetbHidden _array_element)
      (if (not (Variables|/Game/PersoFolder/BP/StarCoins/BP_StarCoins.BP_StarCoins_C|GetSauvegarder _array_element))
        (Rendering|SetActorHiddenInGame _array_element false)
        (Collision|SetCollisionEnabled (Variables|/Game/PersoFolder/BP/StarCoins/BP_StarCoins.BP_StarCoins_C|GetSphere _array_element) "QueryAndPhysics"))))
  (bind _asbp_star_mage_character (Utilities|Casting|CastToBP_StarMageCharacter OtherActor))
  (Variables|/Game/PersoFolder/BP/BP_StarMageCharacter.BP_StarMageCharacter_C|SetKillPlayer _asbp_star_mage_character true)
  (Variables|Default|SetRespawn true)
  (Default|DeathPlayer _asbp_star_mage_character)
  (Utilities|FlowControl|Delay 0.2)
  (Variables|Default|SetRespawn false))

(event OnComponentBeginOverlap(DissolveCollision)
  (params (OverlappedComponent :type Primitive%20Component%20Object%20Reference) (OtherActor :type Actor%20Object%20Reference) (OtherComp :type Primitive%20Component%20Object%20Reference) (OtherBodyIndex :type Integer) (bFromSweep :type Boolean) (SweepResult :type Hit%20Result%20Structure%20%28by%20ref%29))
  (bind _asbp_star_mage_character (Utilities|Casting|CastToBP_StarMageCharacter OtherActor))
  (bind _dissolvev2 (Timeline|Dissolve PlayFromStart)
    (:Update
      (Variables|/Script/Engine.CharacterMovementComponent|SetGravityScale (Variables|/Script/Engine.Character|GetCharacterMovement _asbp_star_mage_character) 0.75)
      (Variables|/Script/Engine.MovementComponent|SetVelocity (Variables|/Script/Engine.Character|GetCharacterMovement _asbp_star_mage_character) (Math|Vector|MakeVector 0.0 0.0 _dissolvev2))
      (Utilities|IsValid (Variables|/Game/PersoFolder/BP/BP_StarMageCharacter.BP_StarMageCharacter_C|GetDissolveMaterial _asbp_star_mage_character)
        (:Is%20Valid
          (Rendering|Material|SetScalarParameterValue (Variables|/Game/PersoFolder/BP/BP_StarMageCharacter.BP_StarMageCharacter_C|GetDissolveMaterial _asbp_star_mage_character) "Dissolve" _dissolvev2 :!class /Script/Engine.MaterialInstanceDynamic))))))

(fn ConstructionScript)