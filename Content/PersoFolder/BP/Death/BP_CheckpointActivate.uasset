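; Checkpoint actor that records player progress when BP_StarMageCharacter overlaps its sphere, unless BP_DeathZone is respawning.
; Hidden BP_StarCoins get flagged as saved on each such overlap.
; A DoOnce, reset after a short delay, registers the checkpoint in BP_ThirdPersonGameMode and stores coin and ring state.
; It also plays a sound, copies saved coins to the character, calls its CreateDissolveMaterial and prints the count.
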(event OnComponentBeginOverlap(SphereCollisionCheckpoint)
  (params (OverlappedComponent :type Primitive%20Component%20Object%20Reference) (OtherActor :type Actor%20Object%20Reference) (OtherComp :type Primitive%20Component%20Object%20Reference) (OtherBodyIndex :type Integer) (bFromSweep :type Boolean) (SweepResult :type Hit%20Result%20Structure%20%28by%20ref%29))
  (bind _returnvalue (Actor|GetActorOfClass "/Game/PersoFolder/BP/Death/BP_DeathZone.BP_DeathZone_C"))
  (if (not (Variables|/Game/PersoFolder/BP/Death/BP_DeathZone.BP_DeathZone_C|GetRespawn _returnvalue))
    (bind _asbp_star_mage_character (Utilities|Casting|CastToBP_StarMageCharacter OtherActor))
    ;[1 1 1] Si au checkpoint l'objet est caché alors lui activer sauvegarder
    (bind _outactors (Actor|GetAllActorsOfClass "/Game/PersoFolder/BP/StarCoins/BP_StarCoins.BP_StarCoins_C"))
    (for _array_element _outactors
      (if (Variables|/Script/Engine.Actor|GetbHidden _array_element)
        (Variables|/Game/PersoFolder/BP/StarCoins/BP_StarCoins.BP_StarCoins_C|SetSauvegarder _array_element true)))
    (Utilities|FlowControl|DoOnce false :!label _label
      (:Completed
        (bind _asbp_third_person_game_mode (Utilities|Casting|CastToBP_ThirdPersonGameMode (Game|GetGameMode)))
        (Variables|/Game/ThirdPerson/Blueprints/BP_ThirdPersonGameMode.BP_ThirdPersonGameMode_C|SetLastCheckpoint _asbp_third_person_game_mode self)
        (Variables|Default|SetSaveCoins (Variables|/Game/PersoFolder/BP/BP_StarMageCharacter.BP_StarMageCharacter_C|GetStarCoinValue _asbp_star_mage_character))
        (Variables|Default|SetsaveRingEquiped (Variables|/Game/PersoFolder/BP/BP_StarMageCharacter.BP_StarMageCharacter_C|GetRingEquiped? _asbp_star_mage_character))
        (Audio|PlaySound2D "/Engine/EditorSounds/GamePreview/EndSimulate.EndSimulate" 1.0 1.0 0.0 0 0)
        (Variables|Default|SetCheckpointOk true)
        (bind _returnvalue_2 (Actor|GetActorOfClass "/Game/PersoFolder/BP/BP_StarMageCharacter.BP_StarMageCharacter_C"))
        (bind _output_get (Variables|/Game/PersoFolder/BP/BP_StarMageCharacter.BP_StarMageCharacter_C|SetSave_Coins_Last_Checkpoint _returnvalue_2 (Variables|Default|GetSaveCoins)))
        (Default|CreateDissolveMaterial _returnvalue_2)
        (Development|PrintString (Utilities|String|ToString(Float) _output_get))
        (Utilities|FlowControl|Delay 0.2)
        (goto _label Reset)))))

(event EventBeginPlay
  (Variables|Default|SetCheckpointOk false))

(fn ConstructionScript)