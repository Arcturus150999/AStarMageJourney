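; BP_PlatformMoveCheckpoint is a moving platform whose path runs between two configurable points, Location1 and Location2.
; The construction script feeds both points into an InterpToMovement component as relative control points, so that component handles the motion.
; The events and MovingPlatform function are empty.
; Unreached leftovers include a duplicate control-point setup and a timeline lerp behind a BP_CheckpointActivate cast, so no checkpoint trigger is active here.
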(event EventBeginPlay)

(event Collision|EventActorBeginOverlap
  (params (OtherActor :type Actor%20Object%20Reference)))

(event EventTick
  (params (DeltaSeconds :type Float%20%28single-precision%29)))

(fn ConstructionScript
  (Variables|/Script/Engine.InterpToMovementComponent|SetControlPoints (Variables|Default|GetInterpToMovement) (Utilities|Array|MakeArray (Utilities|Struct|MakeInterpControlPoint (Variables|Default|GetLocation1) true) (Utilities|Struct|MakeInterpControlPoint (Variables|Default|GetLocation2) true))))

(fn MovingPlatform)